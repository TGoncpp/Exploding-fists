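; Player boxer pawn that weaves and ducks its head and throws jabs and straights at BP_BoxerOpponent.
; Tick moves and rolls the body within bounds, then regenerates stamina; leaning off-center drains stamina, loops a warning sound and changes the aiming dot.
; Punches require being centered and unstunned, enable fist collision and delegate to Jab/Straight components.
; Fist overlaps with the opponent's head send damage, stun and direction to BPC_RecieveDamage, guarded against repeat hits.
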(event OnComponentBeginOverlap(jabCollision)
  (params (OverlappedComponent :type Primitive%20Component%20Object%20Reference) (OtherActor :type Actor%20Object%20Reference) (OtherComp :type Primitive%20Component%20Object%20Reference) (OtherBodyIndex :type Integer) (bFromSweep :type Boolean) (SweepResult :type Hit%20Result%20Structure%20%28by%20ref%29))
  ;[1 1 1] Deal damage on contact
  ;;[1 1 1] Check if head is hit
  (bind _asbp_boxer_opponent (Utilities|Casting|CastToBP_BoxerOpponent OtherActor))
  (if (== (Variables|/Game/pawns/BP_BoxerOpponent.BP_BoxerOpponent_C|GetheadCollision _asbp_boxer_opponent) OtherComp)
    (if (Utilities|Enum|Equal(Enum) (Variables|/Game/Components/BPC_Jab.BPC_Jab_C|Getstate (Variables|Default|GetJabComponent)) "NewEnumerator0")
      (if (not (Variables|Attack|GetheadIsHit))
        (Attack|FindOtherActorandGiveDamage OtherActor (Variables|Attack|GetdamageJab) (Variables|Attack|GetstunFromJab) (Variables|Attack|GetjabVector)))
      (else
        (Variables|Attack|SetheadIsHit false)))))

(event OnComponentBeginOverlap(straightCollision)
  (params (OverlappedComponent :type Primitive%20Component%20Object%20Reference) (OtherActor :type Actor%20Object%20Reference) (OtherComp :type Primitive%20Component%20Object%20Reference) (OtherBodyIndex :type Integer) (bFromSweep :type Boolean) (SweepResult :type Hit%20Result%20Structure%20%28by%20ref%29))
  ;[1 1 1] Deal damage on contact
  ;;[1 1 1] Check if head is hit
  (bind _asbp_boxer_opponent (Utilities|Casting|CastToBP_BoxerOpponent OtherActor))
  (if (== (Variables|/Game/pawns/BP_BoxerOpponent.BP_BoxerOpponent_C|GetheadCollision _asbp_boxer_opponent) OtherComp)
    (if (Utilities|Enum|Equal(Enum) (Variables|/Game/Components/BPC_Straight.BPC_Straight_C|Getstate (Variables|Default|GetStraightComponent)) "NewEnumerator0")
      (if (not (Variables|Attack|GetheadIsHit))
        (Attack|FindOtherActorandGiveDamage OtherActor (Variables|Attack|GetdamageStraight) (Variables|Attack|GetstunFromStraight) (Variables|Attack|GetStraightVector)))
      (else
        (Variables|Attack|SetheadIsHit false)))))

(event Custom|ThrowJab
  (bind _controllerref (Variables|Refrences|GetcontrollerRef))
  (bind _jabcollision (Variables|Default|GetjabCollision))
  (bind _recievedamage (Variables|Default|GetRecieveDamage))
  ;[1 0.4252 0.3794] attack fase
  (Utilities|IsValid _recievedamage
    (:Is%20Valid
      (if (Variables|/Game/Components/BPC_RecieveDamage.BPC_RecieveDamage_C|GetIsstunned _recievedamage)
        (Development|PrintString "still stunned")
        (elif (Variables|center|GetisInCentered)
          (Utilities|IsValid _jabcollision
            (:Is%20Valid
              (Collision|SetCollisionEnabled _jabcollision "QueryAndPhysics")
              (Default|Jab (Variables|Default|GetJabComponent))))
          (else
            (if (== (Game|Player|GetPlayerPawn 0) self)
              (if (Utilities|IsValid _controllerref)
                (Variables|/Game/C_Boxer.C_Boxer_C|SetisAttacking _controllerref false)
                (Default|ClearCommands _controllerref)))
            (Attack|DissableCollision)))))))

(event Custom|ThrowStraight
  (bind _controllerref (Variables|Refrences|GetcontrollerRef))
  (bind _straightcollision (Variables|Default|GetstraightCollision))
  (bind _recievedamage (Variables|Default|GetRecieveDamage))
  ;[1 0.4252 0.3794] attack fase
  (Utilities|IsValid _recievedamage
    (:Is%20Valid
      (if (not (Variables|/Game/Components/BPC_RecieveDamage.BPC_RecieveDamage_C|GetIsstunned _recievedamage))
        (if (Variables|center|GetisInCentered)
          (Utilities|IsValid _straightcollision
            (:Is%20Valid
              (Collision|SetCollisionEnabled _straightcollision "QueryAndPhysics")
              (Default|Straight (Variables|Default|GetStraightComponent))))
          (else
            (if (== (Game|Player|GetPlayerPawn 0) self)
              (if (Utilities|IsValid _controllerref)
                (Variables|/Game/C_Boxer.C_Boxer_C|SetisAttacking _controllerref false)
                (Default|ClearCommands _controllerref)))
            (Attack|DissableCollision)))))))

(event Custom|SetMarkerVisible
  ;[0.6917 0.9661 1] show marker
  (Rendering|SetVisibility (Variables|Default|GetaimingDot) true false))

(event Custom|ResetOffsetsBeforeHitOffset
  ;[1 1 1] When getting hit, reset the offsets before offset hit
  (Default|ResetPosition (Variables|Default|GetStraightComponent))
  (Default|ResetPosition (Variables|Default|GetJabComponent)))

(event EventBeginPlay
  (Refrences|InitialiseRefrences))

(event EventTick
  (params (DeltaSeconds :type Float%20%28single-precision%29))
  ;[1 1 1] HeadMovement
  (movement|HeadMovement DeltaSeconds)
  ;[1 1 1] Check if can attack
  (movement|IsCentered DeltaSeconds)
  (Attack|ResetHitRecord)
  ;[1 1 1] Stamina regeneration
  (Default|Regenerate (Variables|Default|GetStaminaComponent) DeltaSeconds))

(fn ConstructionScript)

(fn HeadMovement
  (params (A :type Float%20%28single-precision%29))
  (bind _controllerref (Variables|Refrences|GetcontrollerRef))
  (if (Utilities|IsValid _controllerref)
    (if (not (Variables|/Game/C_Boxer.C_Boxer_C|GetisAttacking _controllerref))
      (movement|TranslateHead A :!label _label)
      (movement|RotateHead A))
    (else
      (goto _label))))

(fn IsCentered
  (params (time :type Float%20%28double-precision%29))
  (bind _aimingdot (Variables|Default|GetaimingDot))
  (bind _offcentersound (Variables|Default|GetoffCenterSound))
  (if (> (Math|Vector|VectorLength (Variables|movement|GetcoreOffset)) (Variables|center|GetmaxDistanceToCenter))
    (Variables|center|SetisInCentered false)
    (Rendering|Material|SetMaterial _aimingdot 0 "/Engine/VREditor/LaserPointer/LaserPointerMaterial.LaserPointerMaterial")
    ;[1 1 1] Reduce stamina
    (Default|OffCenterPosition (Variables|Default|GetStaminaComponent) time)
    (center|PlaySound)
    (else
      (Variables|center|SetisInCentered true)
      (Rendering|Material|SetMaterial _aimingdot 0 "/Engine/VREditor/LaserPointer/LaserPointerMaterial_Inst.LaserPointerMaterial_Inst")
      (Utilities|IsValid _offcentersound
        (:Is%20Valid
          (if (Audio|Components|Audio|IsPlaying _offcentersound)
            (Audio|Components|Audio|Stop _offcentersound)))))))

(fn RotateHead
  (params (A :type Float%20%28double-precision%29))
  (bind _body (Variables|Default|Getbody))
  (Transformation|SetRelativeRotation _body (Math|Rotator|MakeRotator (* (.y (Variables|/Script/Engine.SceneComponent|GetRelativeLocation _body)) (Variables|movement|GetduckOnSideMovementFactor)) 0.0 0.0) true false))

(fn TranslateHead
  (params (time :type Float%20%28double-precision%29))
  (bind _horizontalspeed (Variables|movement|GethorizontalSpeed))
  (bind _verticalspeed (Variables|movement|GetverticalSpeed))
  (bind _inputvector (Variables|movement|GetinputVector))
  (bind _returnvalue (* time _inputvector))
  (bind _returnvalue_2 (* (.z _returnvalue) _verticalspeed))
  (bind _returnvalue_3 (* (.y _returnvalue) _horizontalspeed))
  (bind _returnvalue_4 (Math|Vector|MakeVector (.x _returnvalue) _returnvalue_3 _returnvalue_2))
  (if (and (<= (Math|Float|Absolute(Float) (.y (+ _returnvalue_4 (Variables|movement|GetcoreOffset)))) (Variables|movement|GetMaxWeaveLength)) (and (>= (.z (+ _returnvalue_4 (Variables|movement|GetcoreOffset))) (Variables|movement|GetlowestZposition)) (<= (.z (+ _returnvalue_4 (Variables|movement|GetcoreOffset))) (Variables|movement|GetmaxHeight))))
    (bind _output_get (Variables|movement|SetcoreOffset (+ _returnvalue_4 (Variables|movement|GetcoreOffset))))
    (Transformation|SetRelativeLocation (Variables|Default|Getbody) _output_get true false)))

(fn FindOtherActorandGiveDamage
  (params (target :type Object%20Object%20Reference) (damage :type Float%20%28double-precision%29) (stunTime :type Float%20%28double-precision%29) (punchDir :type Vector))
  (if (!= target self)
    (bind _asbp_boxer_opponent (Utilities|Casting|CastToBP_BoxerOpponent target))
    (if (Utilities|IsValid (Actor|GetComponentbyClass _asbp_boxer_opponent "/Game/Components/BPC_RecieveDamage.BPC_RecieveDamage_C"))
      (Class|DealDamage|DealDamage(Message) (Actor|GetComponentbyClass _asbp_boxer_opponent "/Game/Components/BPC_RecieveDamage.BPC_RecieveDamage_C") damage self stunTime punchDir)
      (Variables|Attack|SetheadIsHit true)
      (else
        (Development|PrintString "This actor doesnt have the BPC_RecieveDamageComponent" true true "(R=0.000000,G=0.660000,B=1.000000,A=1.000000)" 12.0)))))

(fn DissableCollision
  (Collision|SetCollisionEnabled (Variables|Default|GetjabCollision) "NoCollision")
  (Collision|SetCollisionEnabled (Variables|Default|GetstraightCollision) "NoCollision"))

(fn ResetHitRecord
  (if (Variables|Attack|GetheadIsHit)
    (if (and (not (Utilities|Enum|Equal(Enum) (Variables|/Game/Components/BPC_Jab.BPC_Jab_C|Getstate (Variables|Default|GetJabComponent)) "NewEnumerator0")) (not (Utilities|Enum|Equal(Enum) (Variables|/Game/Components/BPC_Straight.BPC_Straight_C|Getstate (Variables|Default|GetStraightComponent)) "NewEnumerator0")))
      (Variables|Attack|SetheadIsHit false))))

(fn MoveHeadtoCenter
  (params (time :type Float%20%28double-precision%29) (dodgedLeft :type Boolean))
  (bind _isincentered (Variables|center|GetisInCentered))
  (if _isincentered
    (Variables|movement|SetinputVector "0, 0, 0")
    (elif dodgedLeft
      (Variables|movement|SetinputVector (Math|Vector|MakeVector 0.0 (* (LocalVariables|GetmoveSpeed) -1.0) 0.0))
      (else
        (Variables|movement|SetinputVector (Math|Vector|MakeVector 0.0 (LocalVariables|GetmoveSpeed) 0.0)))))
  (return _isincentered))

(fn InitialiseRefrences
  (bind _straightcomponent (Variables|Default|GetStraightComponent))
  (bind _headvisual (Variables|Default|GetheadVisual))
  (bind _jabcomponent (Variables|Default|GetJabComponent))
  ;[0.5028 0.8271 1] enable mainInput mapping
  (Variables|movement|SetCenterPosition (Transformation|GetWorldLocation (Variables|Default|Getcore)))
  ;[0.5028 0.8271 1] Get refrence off controller
  (bind _asc_boxer (Utilities|Casting|CastToC_Boxer (Game|GetPlayerController 0))
    (:then
      (Variables|Refrences|SetcontrollerRef _asc_boxer))
    (:CastFailed
      (Development|PrintString "Failed to load controller" true true "(R=1.000000,G=0.083296,B=0.091253,A=1.000000)" 2e+01)
      (Development|PrintString (Utilities|GetDisplayName _asc_boxer))))
  ;[0.5028 0.8271 1] Initialise Left AttackComponents
  (Variables|/Game/Components/BPC_Jab.BPC_Jab_C|Setfist _jabcomponent (Variables|Default|GetleftFist1))
  (Default|SetControllerRef _jabcomponent (Variables|Refrences|GetcontrollerRef))
  (Default|SetCameraRef _jabcomponent _headvisual)
  ;[0.5028 0.8271 1] Initialise Right AttackComponents
  (Variables|/Game/Components/BPC_Straight.BPC_Straight_C|Setfist _straightcomponent (Variables|Default|GetrightFist))
  (Default|SetControllerRef _straightcomponent (Variables|Refrences|GetcontrollerRef))
  (Default|SetHeadRef _straightcomponent _headvisual)
  ;[0.548 0.9421 1] Init dealDamage comp
  (Default|SetStartValues (Variables|Default|GetRecieveDamage) (Variables|Default|Getcore) false (Variables|Default|GetheadVisual) self)
  ;[0.5533 0.8602 1] disable collision off fists
  (Attack|DissableCollision)
  (Default|LoadHud (Variables|Default|GetStaminaComponent)))

(fn SetVerticaleSpeed
  (params (isDisabled :type Boolean))
  (if isDisabled
    (Variables|movement|SetverticalSpeed 0.0)
    (else
      (Variables|movement|SetverticalSpeed 1.1e+02))))

(fn SetHorizontalSpeed
  (params (disable :type Boolean))
  (if disable
    (Variables|movement|SethorizontalSpeed 0.0)
    (else
      (Variables|movement|SethorizontalSpeed 5e+01))))

(fn DisableSound
  (Utilities|IsValid (Variables|Default|GetoffCenterSound)
    (:Is%20Valid
      (if (Audio|Components|Audio|IsPlaying (Variables|Default|GetoffCenterSound))
        (Audio|Components|Audio|Stop (Variables|Default|GetoffCenterSound))
        (else
          (Variables|Default|SetoffCenterSound 0))))))

(fn PlaySound
  (Utilities|IsValid (Variables|Default|GetoffCenterSound)
    (:Is%20Valid
      (if (not (Audio|Components|Audio|IsPlaying (Variables|Default|GetoffCenterSound)))
        (Audio|Components|Audio|Play (Variables|Default|GetoffCenterSound) 0.0)))
    (:Is%20Not%20Valid
      (bind _returnvalue (Audio|SpawnSound2D "/Game/StarterContent/Audio/Fire01.Fire01" 1.0 1.0 0.0 0))
      (Variables|Default|SetoffCenterSound _returnvalue))))

(fn ClampMovement
  (params (InVec :type Vector))
  (bind (_x _y _z) (Math|Vector|BreakVector InVec))
  (if (> (Math|Float|Absolute(Float) (/ _y _z)) 0.0)
    (return (Math|Vector|MakeVector 0.0 _y 0.0))
    (else
      (return (Math|Vector|MakeVector 0.0 0.0 _z)))))