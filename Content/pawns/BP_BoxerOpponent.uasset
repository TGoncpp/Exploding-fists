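; AI boxer opponent pawn that weaves, ducks and throws jabs, straights and hooks.
; While its AI controller allows movement, Tick moves the head within bounds, drains stamina off-center and regenerates it.
; Punch components drive the fists: jab and straight require a centered head, hook shares jab collision, and stun cancels a throw.
; Fist overlaps with a boxer's head send damage through BPC_RecieveDamage; a dynamic material colors the head by health.
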(event OnComponentBeginOverlap(jabCollision)
  (params (OverlappedComponent :type Primitive%20Component%20Object%20Reference) (OtherActor :type Actor%20Object%20Reference) (OtherComp :type Primitive%20Component%20Object%20Reference) (OtherBodyIndex :type Integer) (bFromSweep :type Boolean) (SweepResult :type Hit%20Result%20Structure%20%28by%20ref%29))
  (bind _jabcomponent (Variables|Default|GetJabComponent))
  ;[1 1 1] Deal damage on contact
  ;;[1 1 1] Check if head is hit
  (bind _asbp_boxer (Utilities|Casting|CastToBP_Boxer OtherActor))
  (if (== (Variables|/Game/pawns/BP_Boxer.BP_Boxer_C|GetheadCollision _asbp_boxer) OtherComp)
    (Utilities|IsValid _jabcomponent
      (:Is%20Valid
        (if (or (Utilities|Enum|Equal(Enum) (Variables|/Game/Components/BPC_Jab.BPC_Jab_C|Getstate _jabcomponent) "NewEnumerator0") (Class|HookAttackComp|IsThrowing (Variables|Default|GetHookComponent)))
          (if (not (Variables|Attack|GetheadIsHit))
            (CallFunction|FindOtherActorandGiveDamage OtherActor (Variables|Attack|GetdamageJab) (Variables|Attack|GetstunFromJab) (Variables|Attack|GetjabVector))
            (Utilities|IsValid (Variables|Default|GetjabCollision)
              (:Is%20Valid
                (Collision|SetCollisionEnabled (Variables|Default|GetstraightCollision) "NoCollision"))))
          (else
            (Variables|Attack|SetheadIsHit false)))))))

(event OnComponentBeginOverlap(straightCollision)
  (params (OverlappedComponent :type Primitive%20Component%20Object%20Reference) (OtherActor :type Actor%20Object%20Reference) (OtherComp :type Primitive%20Component%20Object%20Reference) (OtherBodyIndex :type Integer) (bFromSweep :type Boolean) (SweepResult :type Hit%20Result%20Structure%20%28by%20ref%29))
  (bind _straightcollision (Variables|Default|GetstraightCollision))
  (bind _straightcomponent (Variables|Default|GetStraightComponent))
  ;[1 1 1] Deal damage on contact
  ;;[1 1 1] Check if head is hit
  (bind _asbp_boxer (Utilities|Casting|CastToBP_Boxer OtherActor))
  (if (== (Variables|/Game/pawns/BP_Boxer.BP_Boxer_C|GetheadCollision _asbp_boxer) OtherComp)
    (Utilities|IsValid _straightcomponent
      (:Is%20Valid
        (if (Utilities|Enum|Equal(Enum) (Variables|/Game/Components/BPC_Straight.BPC_Straight_C|Getstate _straightcomponent) "NewEnumerator0")
          (if (not (Variables|Attack|GetheadIsHit))
            (CallFunction|FindOtherActorandGiveDamage OtherActor (Variables|Attack|GetdamageStraight) (Variables|Attack|GetstunFromStraight) (Variables|Attack|GetStraightVector))
            (Utilities|IsValid _straightcollision
              (:Is%20Valid
                (Collision|SetCollisionEnabled _straightcollision "NoCollision"))))
          (else
            (Variables|Attack|SetheadIsHit false)))))))

(event Custom|ThrowJab
  (bind _jabcollision (Variables|Default|GetjabCollision))
  (bind _recievedamage (Variables|Default|GetRecieveDamage))
  ;[1 0.4252 0.3794] attack fase
  (Utilities|IsValid _recievedamage
    (:Is%20Valid
      (if (Variables|/Game/Components/BPC_RecieveDamage.BPC_RecieveDamage_C|GetIsstunned _recievedamage)
        (Variables|/Game/Components/BPC_RecieveDamage.BPC_RecieveDamage_C|SetIsstunned _recievedamage false)
        (elif (Variables|center|GetisInCentered)
          (Utilities|IsValid _jabcollision
            (:Is%20Valid
              (Collision|SetCollisionEnabled _jabcollision "QueryAndPhysics")
              (Default|Jab (Variables|Default|GetJabComponent))
              (Audio|PlaySound2D "/Engine/VREditor/Sounds/UI/Drop_Item_From_ContentBrowser.Drop_Item_From_ContentBrowser" 1.0 1.0 0.0 0 0)))
          (else
            (CallFunction|DissableCollision)))))))

(event Custom|UpdateColor
  (CallFunction|UpdateMaterialColor))

(event Custom|SetMarkerVisible
  (bind _aimingdot (Variables|Default|GetaimingDot))
  ;[0.6917 0.9661 1] show marker
  (Utilities|IsValid _aimingdot
    (:Is%20Valid
      (Rendering|SetVisibility _aimingdot true false))))

(event Custom|ResetOffsetsBeforeHitOffset
  (bind _straightcomponent (Variables|Default|GetStraightComponent))
  (bind _jabcomponent (Variables|Default|GetJabComponent))
  ;[1 1 1] When getting hit, reset the offsets before offset hit
  (Utilities|IsValid _straightcomponent
    (:Is%20Valid
      (Default|ResetPosition _straightcomponent)
      (Utilities|IsValid _jabcomponent
        (:Is%20Valid
          (Default|ResetPosition _jabcomponent))))))

(event Custom|ThrowStraight
  (bind _straightcollision (Variables|Default|GetstraightCollision))
  (bind _recievedamage (Variables|Default|GetRecieveDamage))
  ;[1 0.4252 0.3794] attack fase
  (Utilities|IsValid _recievedamage
    (:Is%20Valid
      (if (Variables|/Game/Components/BPC_RecieveDamage.BPC_RecieveDamage_C|GetIsstunned _recievedamage)
        (Variables|/Game/Components/BPC_RecieveDamage.BPC_RecieveDamage_C|SetIsstunned _recievedamage false)
        (elif (Variables|center|GetisInCentered)
          (Utilities|IsValid _straightcollision
            (:Is%20Valid
              (Collision|SetCollisionEnabled _straightcollision "QueryAndPhysics")
              (Default|Straight (Variables|Default|GetStraightComponent))
              (Audio|PlaySound2D "/Engine/VREditor/Sounds/UI/Drop_Item_From_ContentBrowser.Drop_Item_From_ContentBrowser" 1.0 1.0 0.0 0 0)))
          (else
            (CallFunction|DissableCollision)))))))

(event Custom|ThrowHook
  (bind _jabcollision (Variables|Default|GetjabCollision))
  (bind _recievedamage (Variables|Default|GetRecieveDamage))
  ;[1 0.4252 0.3794] attack fase
  (Utilities|IsValid _recievedamage
    (:Is%20Valid
      (if (Variables|/Game/Components/BPC_RecieveDamage.BPC_RecieveDamage_C|GetIsstunned _recievedamage)
        (Variables|/Game/Components/BPC_RecieveDamage.BPC_RecieveDamage_C|SetIsstunned _recievedamage false)
        (else
          (Utilities|IsValid _jabcollision
            (:Is%20Valid
              (Collision|SetCollisionEnabled _jabcollision "QueryAndPhysics")
              (Class|HookAttackComp|Hook (Variables|Default|GetHookComponent))
              (Audio|PlaySound2D "/Engine/VREditor/Sounds/UI/Drop_Item_From_ContentBrowser.Drop_Item_From_ContentBrowser" 1.0 1.0 0.0 0 0))))))))

(event EventBeginPlay
  (CallFunction|InitialiseRefrences)
  (Class|HookAttackComp|InitializeComponents (Variables|Default|GetHookComponent) (Variables|Default|Getcore) (Variables|Default|GetleftFist1)))

(event EventTick
  (params (DeltaSeconds :type Float%20%28single-precision%29))
  (bind _aicontroller (Variables|refrences|GetAIController))
  (bind _staminacomponent (Variables|Default|GetStaminaComponent))
  (Utilities|IsValid _aicontroller
    (:Is%20Valid
      (if (Variables|/Game/AI/C_AIController.C_AIController_C|GetisMoveAble _aicontroller)
        ;[1 1 1] HeadMovement
        (CallFunction|HeadMovement DeltaSeconds)
        ;[1 1 1] Check if can attack
        (CallFunction|IsCentered DeltaSeconds)
        (CallFunction|ResetHitRecord)
        ;[1 1 1] Stamina regeneration
        (if (Utilities|IsValid _staminacomponent)
          (Default|Regenerate _staminacomponent DeltaSeconds))))))

(fn ConstructionScript
  (bind _returnvalue (Rendering|Material|CreateDynamicMaterialInstance (Variables|Default|GetheadVisual) 0 "/Game/Textures/BPM_HealtColorBase_Inst.BPM_HealtColorBase_Inst" "color" :!class /Script/Engine.PrimitiveComponent))
  (Variables|Default|SetHPColor _returnvalue)
  (CallFunction|UpdateMaterialColor))

(fn HeadMovement
  (params (A :type Float%20%28single-precision%29))
  (CallFunction|TranslateHead A)
  (CallFunction|RotateHead A))

(fn GetZValueforMovement
  (params (totalSideOffset :type Float%20%28double-precision%29) (currentHeightOffset :type Float%20%28double-precision%29))
  (return 0.0))

(fn IsCentered
  (params (time :type Float%20%28double-precision%29))
  (bind _aimingdot (Variables|Default|GetaimingDot))
  (bind _staminacomponent (Variables|Default|GetStaminaComponent))
  (bind _returnvalue (Utilities|IsValid _aimingdot))
  (if (> (Math|Vector|VectorLength (Variables|movement|GetcoreOffset)) (Variables|center|GetmaxDistanceToCenter))
    (Variables|center|SetisInCentered false)
    (if _returnvalue
      (Rendering|Material|SetMaterial _aimingdot 0 "/Engine/VREditor/LaserPointer/LaserPointerMaterial.LaserPointerMaterial")
      ;[1 1 1] Reduce stamina
      (if (Utilities|IsValid _staminacomponent)
        (Default|OffCenterPosition _staminacomponent time)))
    (else
      (Variables|center|SetisInCentered true)
      (if _returnvalue
        (Rendering|Material|SetMaterial _aimingdot 0 "/Engine/VREditor/LaserPointer/LaserPointerMaterial_Inst.LaserPointerMaterial_Inst")))))

(fn RotateHead
  (params (A :type Float%20%28double-precision%29))
  (bind _body (Variables|Default|Getbody))
  (if (Utilities|IsValid _body)
    (Transformation|SetRelativeRotation _body (Math|Rotator|MakeRotator (* (.y (Variables|/Script/Engine.SceneComponent|GetRelativeLocation _body)) (Variables|movement|GetduckOnSideMovementFactor)) 0.0 0.0) true false)))

(fn TranslateHead
  (params (time :type Float%20%28double-precision%29))
  (bind _horizontalspeed (Variables|movement|GethorizontalSpeed))
  (bind _verticalspeed (Variables|movement|GetverticalSpeed))
  (bind _inputvector (Variables|movement|GetinputVector))
  (bind _returnvalue (* time _inputvector))
  (bind _returnvalue_2 (* (.z _returnvalue) _verticalspeed))
  (bind _returnvalue_3 (* (.y _returnvalue) _horizontalspeed))
  (bind _returnvalue_4 (Math|Vector|MakeVector (.x _returnvalue) _returnvalue_3 _returnvalue_2))
  (if (and (<= (Math|Float|Absolute(Float) (.y (+ _returnvalue_4 (Variables|movement|GetcoreOffset)))) (Variables|movement|GetMaxWeaveLength)) (and (>= (.z (+ _returnvalue_4 (Variables|movement|GetcoreOffset))) (Variables|movement|GetlowestZposition)) (<= (.z (+ _returnvalue_4 (Variables|movement|GetcoreOffset))) (Variables|movement|GetmaxHeight))))
    (bind _output_get (Variables|movement|SetcoreOffset (+ _returnvalue_4 (Variables|movement|GetcoreOffset))))
    (Transformation|SetRelativeLocation (Variables|Default|Getbody) _output_get true false)))

(fn FindOtherActorandGiveDamage
  (params (target :type Object%20Object%20Reference) (damage :type Float%20%28double-precision%29) (stunTime :type Float%20%28double-precision%29) (punchDir :type Vector))
  (if (!= target self)
    (bind _asbp_boxer (Utilities|Casting|CastToBP_Boxer target))
    (if (Utilities|IsValid (Actor|GetComponentbyClass _asbp_boxer "/Game/Components/BPC_RecieveDamage.BPC_RecieveDamage_C"))
      (Class|DealDamage|DealDamage(Message) (Actor|GetComponentbyClass _asbp_boxer "/Game/Components/BPC_RecieveDamage.BPC_RecieveDamage_C") damage self stunTime punchDir)
      (Variables|Attack|SetheadIsHit true)
      (else
        (Development|PrintString "This actor doesnt have the BPC_RecieveDamageComponent" true true "(R=0.000000,G=0.660000,B=1.000000,A=1.000000)" 12.0)))))

(fn DissableCollision
  (Collision|SetCollisionEnabled (Variables|Default|GetjabCollision) "NoCollision")
  (Collision|SetCollisionEnabled (Variables|Default|GetstraightCollision) "NoCollision"))

(fn ResetHitRecord
  (if (Variables|Attack|GetheadIsHit)
    (if (and (not (Utilities|Enum|Equal(Enum) (Variables|/Game/Components/BPC_Jab.BPC_Jab_C|Getstate (Variables|Default|GetJabComponent)) "NewEnumerator0")) (and (not (Utilities|Enum|Equal(Enum) (Variables|/Game/Components/BPC_Straight.BPC_Straight_C|Getstate (Variables|Default|GetStraightComponent)) "NewEnumerator0")) (not (Class|HookAttackComp|IsThrowing (Variables|Default|GetHookComponent)))))
      (Variables|Attack|SetheadIsHit false))))

(fn MoveHeadtoCenter
  (params (time :type Float%20%28double-precision%29) (dodgedLeft :type Boolean))
  (bind _isincentered (Variables|center|GetisInCentered))
  (if _isincentered
    (Variables|movement|SetinputVector "0, 0, 0")
    (elif dodgedLeft
      (Variables|movement|SetinputVector (Math|Vector|MakeVector 0.0 (* (LocalVariables|GetmoveSpeed) -1.0) 0.0))
      (else
        (Variables|movement|SetinputVector (Math|Vector|MakeVector 0.0 (LocalVariables|GetmoveSpeed) 0.0)))))
  (return _isincentered))

(fn InitialiseRefrences
  (bind _straightcomponent (Variables|Default|GetStraightComponent))
  (bind _headvisual (Variables|Default|GetheadVisual))
  (bind _jabcomponent (Variables|Default|GetJabComponent))
  ;[0.5028 0.8271 1] enable mainInput mapping
  (Variables|movement|SetCenterPosition (Transformation|GetWorldLocation (Variables|Default|Getcore)))
  ;[0.5028 0.8271 1] Get refrence off controller
  (bind _asc_aicontroller (Utilities|Casting|CastToC_AIController (Pawn|GetController))
    (:then
      (Variables|refrences|SetAIController _asc_aicontroller))
    (:CastFailed
      (Development|PrintString "Failed to load controller" true true "(R=1.000000,G=0.083296,B=0.091253,A=1.000000)" 2e+01)))
  ;[0.5028 0.8271 1] Initialise Left AttackComponents
  (Variables|/Game/Components/BPC_Jab.BPC_Jab_C|Setfist _jabcomponent (Variables|Default|GetleftFist1))
  (Default|SetCameraRef _jabcomponent _headvisual)
  ;[0.5028 0.8271 1] Initialise Right AttackComponents
  (Variables|/Game/Components/BPC_Straight.BPC_Straight_C|Setfist _straightcomponent (Variables|Default|GetrightFist))
  (Default|SetHeadRef _straightcomponent _headvisual)
  ;[0.548 0.9421 1] Init dealDamage comp
  (Default|SetStartValues (Variables|Default|GetRecieveDamage) (Variables|Default|Getcore) false (Variables|Default|GetheadVisual) self)
  ;[0.5533 0.8602 1] disable collision off fists
  (CallFunction|DissableCollision)
  (Default|LoadHud (Variables|Default|GetStaminaComponent)))

(fn UpdateMaterialColor
  (bind _healthcurve (Variables|Default|GethealthCurve))
  (bind _hpcolor (Variables|Default|GetHPColor)
    (:then
      (Rendering|Material|SetVectorParameterValue _hpcolor "color" (Math|Color|SelectColor (Math|Curves|GetLinearColorValue _healthcurve (Variables|/Game/Components/BPC_RecieveDamage.BPC_RecieveDamage_C|Gethealth (Variables|Default|GetRecieveDamage))) "(R=0.140278,G=0.475440,B=0.841667,A=1.000000)" (Utilities|IsValid _healthcurve)) :!class /Script/Engine.MaterialInstanceDynamic))
    (:else)))