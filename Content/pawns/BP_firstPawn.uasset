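; BP_firstPawn is a player pawn that moves on the horizontal plane from Enhanced Input.
; On BeginPlay it adds the IMC_Main mapping context to its player controller's input subsystem.
; Tick polls IA_PlayerMovement, swaps its axes into world X/Y and clamps the length to one so diagonals are not faster.
; It then applies a swept world offset scaled by Speed and delta time.
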(event EventBeginPlay
  ;[1 1 1] enable mainInput mapping
  (bind _asplayer_controller (Utilities|Casting|CastToPlayerController (Pawn|GetController)))
  (Utilities|IsValid (PlayerController|LocalPlayerSubsystems|GetEnhancedInputLocalPlayerSubsystem _asplayer_controller)
    (:Is%20Valid
      (Input|AddMappingContext (PlayerController|LocalPlayerSubsystems|GetEnhancedInputLocalPlayerSubsystem _asplayer_controller) "/Game/Input/IMC_Main.IMC_Main" 0 "(bIgnoreAllPressedKeysUntilRelease=True,bForceImmediately=False)"))))

(event EventTick
  (params (DeltaSeconds :type Float%20%28single-precision%29))
  (bind _returnvalue (Input|EnhancedActionValues|GetIA_PlayerMovement))
  (Transformation|AddActorWorldOffset (* (* DeltaSeconds (Math|Vector|ClampVectorSize (Math|Vector|MakeVector (.y _returnvalue) (.x _returnvalue) 0.0) 0.0 1.0)) (Variables|pawnMovement|Getspeed)) true))

(fn ConstructionScript)