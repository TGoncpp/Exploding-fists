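; Damage-receiving component for boxers that handles health, hit reactions and ending the round when health runs out.
; DealDamage plays hit effects, subtracts health, adds stun time and sets AI controllers to stun; BeginPlay creates both health bar widgets.
; While stunned, Tick offsets the body along the punch vector up to a maximum and yaws the head, then eases both back.
; CanAttack requires the boxer to be unstunned and centered.
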(event Custom|SetStartValues
  (params (bodyMeshRef :type Static%20Mesh%20Component%20Object%20Reference) (isPlayer :type Boolean) (headMeshRef :type Static%20Mesh%20Component%20Object%20Reference) (boxer :type BP%20Boxer%20Base%20Object%20Reference))
  ;[0.5097 0.9741 1] get pawn refrence
  (if (Utilities|IsValid bodyMeshRef)
    (Variables|Default|SetbodyRef bodyMeshRef)
    (if (Utilities|IsValid headMeshRef)
      (Variables|Default|SetheadRef headMeshRef)
      (Variables|refrences|SetownerRef boxer)
      (else
        (Development|PrintString "Invallid startvalue" true true "(R=0.000000,G=0.660000,B=1.000000,A=1.000000)" 2e+01 :!label _label)))
    (else
      (goto _label))))

(event Custom|ApplyKnockback
  (bind _bodyref (Variables|Default|GetbodyRef))
  ;[1 1 1] set resetPosition before applying knockback
  (if (Utilities|IsValid _bodyref)
    (Variables|knockback|SetstartPos (Transformation|GetWorldLocation _bodyref))
    (bind _asc_aicontroller (Utilities|Casting|CastToC_AIController (AI|GetAIController (Components|GetOwner))))
    (Default|SettoStun _asc_aicontroller)
    (else
      (Development|PrintString "Failed to load core" true true "(R=0.000000,G=0.660000,B=1.000000,A=1.000000)" 1e+01))))

(event EventBeginPlay
  ;[1 1 1] set widget for player and enemy
  (bind _returnvalue (UserInterface|CreateWidget "/Game/HUD/HUD_OppHealthBar.HUD_OppHealthBar_C"))
  (UserInterface|Viewport|AddtoViewport _returnvalue 0)
  (bind _returnvalue_2 (UserInterface|CreateWidget "/Game/HUD/HUD_PlayerHealthBar.HUD_PlayerHealthBar_C"))
  (UserInterface|Viewport|AddtoViewport _returnvalue_2 0)
  (Variables|recover|SetrecoverSpeed (* (Variables|knockback|GetknockBackSpeed) 0.35)))

(event EventTick
  (params (DeltaSeconds :type Float%20%28single-precision%29))
  ;[1 1 1] Knockback/recover
  (if (> (Variables|knockback|GetstunTime) 0.0)
    (CallFunction|Knockback DeltaSeconds)
    (elif (Variables|knockback|GetIsstunned)
      (CallFunction|RecoverPosition DeltaSeconds))))

(event EventDealDamage
  (params (damage :type Float%20%28double-precision%29) (attacker :type BP%20Boxer%20Base%20Object%20Reference) (stunTime :type Float%20%28double-precision%29) (punchVector :type Vector :default "0, 0, 0"))
  ;[1 1 1] Recieve damage
  (if (!= attacker self)
    (Variables|knockback|SetIsstunned true)
    (CallFunction|HitEffects)
    (bind _output_get (CallFunction|UpdateHealthandStun damage stunTime))
    (Variables|knockback|SetknockbackDirection punchVector)
    (CallFunction|ApplyKnockback)
    (if (<= _output_get 0.0)
      (bind _asfight_mode (Utilities|Casting|CastTofightMode (Game|GetGameMode)))
      (bind _asbp_boxer (Utilities|Casting|CastToBP_Boxer (Variables|refrences|GetownerRef))
        (:then
          (Default|DisableSound _asbp_boxer)
          (Default|Nextround _asfight_mode true))
        (:CastFailed
          (Default|Nextround _asfight_mode false))))))

(fn Knockback
  (params (A :type Float%20%28single-precision%29))
  (bind _knockbackspeed (Variables|knockback|GetknockBackSpeed))
  (bind _headref (Variables|Default|GetheadRef))
  (bind _knockbackdirection (Variables|knockback|GetknockbackDirection))
  (bind _bodyref (Variables|Default|GetbodyRef))
  (bind _returnvalue (* A _knockbackspeed))
  (bind _returnvalue_2 (* _returnvalue _knockbackdirection))
  (if (<= (Math|Vector|VectorLength (+ _returnvalue_2 (Variables|knockback|GettotalOffset))) (Variables|knockback|GetmaxOffset))
    (Utilities|IsValid _bodyref
      (:Is%20Valid
        (Transformation|AddLocalOffset _bodyref _returnvalue_2 true false)
        (Variables|knockback|SettotalOffset (+ (Variables|knockback|GettotalOffset) _returnvalue_2))
        (Variables|knockback|SetstunTime (- (Variables|knockback|GetstunTime) A))
        (Utilities|IsValid _headref
          (:Is%20Valid
            (Transformation|SetRelativeRotation _headref (Math|Rotator|MakeRotator 0.0 0.0 (* (.y (Variables|knockback|GetknockbackDirection)) 1.8e+02)) true false)))))
    (else
      ;[1 1 1] if stun time close to zero, reset
      (bind _output_get (Variables|knockback|SetstunTime (- A (Variables|knockback|GetstunTime))))
      (if (<= _output_get 0.0)
        (Variables|knockback|SetstunTime 0.0)))))

(fn RecoverPosition
  (params (time :type Float%20%28double-precision%29))
  (CallFunction|RecoverPosTranslation time)
  (CallFunction|RecoverRotation time)
  (CallFunction|CheckifRecovered))

(fn RecoverPosTranslation
  (params (time :type Float%20%28double-precision%29))
  (bind _bodyref (Variables|Default|GetbodyRef))
  (bind _recoverspeed (Variables|recover|GetrecoverSpeed))
  (bind _knockbackdirection (Variables|knockback|GetknockbackDirection))
  (bind _bodyref_2 (Variables|Default|GetbodyRef))
  (bind _returnvalue (* time _recoverspeed))
  (bind _returnvalue_2 (* _returnvalue _knockbackdirection))
  (bind _returnvalue_3 (Math|Vector|NegateVector _returnvalue_2))
  (if (Math|Float|InRange(Float) (Math|Vector|VectorLengthSquared (+ _returnvalue_3 (Variables|knockback|GettotalOffset))) 0.0 1e+02)
    ;[1 1 1] if reached startposition, Reset to start
    (Utilities|IsValid _bodyref
      (:Is%20Valid
        (Transformation|AddLocalOffset _bodyref (Math|Vector|NegateVector (Variables|knockback|GettotalOffset)) false true)
        (Variables|knockback|SettotalOffset "0, 0, 0")))
    (else
      ;[1 1 1] Recover position
      (Utilities|IsValid _bodyref_2
        (:Is%20Valid
          (Transformation|AddLocalOffset _bodyref_2 _returnvalue_3 true false)
          (Variables|knockback|SettotalOffset (+ (Variables|knockback|GettotalOffset) _returnvalue_3))))))
  (return))

(fn RecoverRotation
  (params (InputPin :type Float%20%28double-precision%29))
  (bind _headref (Variables|Default|GetheadRef))
  (bind _relativerotation (Variables|/Script/Engine.SceneComponent|GetRelativeRotation _headref))
  (if (> (Math|Float|Absolute(Float) (.yaw _relativerotation)) 0.5)
    (Transformation|SetRelativeRotation _headref (Math|Rotator|MakeRotator 0.0 0.0 (- (.yaw _relativerotation) (* (.yaw _relativerotation) (* InputPin (Variables|recover|GetrotationRecoverSpeed))))) true false)
    (else
      (Transformation|SetRelativeRotation _headref "0, 0, 0" false false))))

(fn CheckifRecovered
  (if (Variables|knockback|GetIsstunned)
    (if (and (Utilities|Operators|EqualEqual :A (Variables|knockback|GettotalOffset)) (Utilities|Operators|EqualEqual :A (Variables|/Script/Engine.SceneComponent|GetRelativeRotation (Variables|Default|GetheadRef))))
      (Variables|knockback|SetIsstunned false))))

(fn CanAttack
  (bind _ownerref (Variables|refrences|GetownerRef))
  (bind _asbp_boxer (Utilities|Casting|CastToBP_Boxer _ownerref)
    (:then
      (return (and (not (Variables|knockback|GetIsstunned)) (Variables|/Game/pawns/BP_Boxer.BP_Boxer_C|GetisInCentered _asbp_boxer))))
    (:CastFailed
      (bind _asbp_boxer_opponent (Utilities|Casting|CastToBP_BoxerOpponent _ownerref))
      (return (and (not (Variables|knockback|GetIsstunned)) (Variables|/Game/pawns/BP_BoxerOpponent.BP_BoxerOpponent_C|GetisInCentered _asbp_boxer_opponent))))))

(fn HitEffects
  (Audio|PlaySound2D "/Game/StarterContent/Audio/Explosion01.Explosion01" 1.0 1.0 0.0 0 0)
  (Effects|SpawnEmitteratLocation "/Game/StarterContent/Particles/P_Explosion.P_Explosion" (Transformation|GetWorldLocation (Variables|Default|GetheadRef))))

(fn UpdateHealthandStun
  (params (B :type Float%20%28double-precision%29) (A :type Float%20%28double-precision%29))
  (bind _output_get (Variables|Default|Sethealth (- (Variables|Default|Gethealth) B)))
  (Variables|knockback|SetstunTime (+ A (Variables|knockback|GetstunTime)))
  (bind _asbp_boxer_opponent (Utilities|Casting|CastToBP_BoxerOpponent (Variables|refrences|GetownerRef))
    (:then
      (Default|UpdateColor _asbp_boxer_opponent))
    (:CastFailed
      _))
  (return _output_get))