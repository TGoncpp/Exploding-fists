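; Jab attack component that procedurally animates a punch by moving the Fist and Head along local Y.
; Jab() plays a sound and starts a Tick-driven state machine: wind-up with camera shift, punch, delay, then retract.
; Swept offsets are accumulated to test each phase's distance, with return speeds derived from forward speeds.
; After retraction, both parts teleport back by their accumulated offsets and the controller's IsAttacking flag clears.
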(event Custom|Jab
  ;[1 0.3198 0.3198] Start attack
  (Variables|attackValues|Setstate "NewEnumerator4")
  (Audio|PlaySound2D "/Engine/VREditor/Sounds/UI/Drop_Item_From_ContentBrowser.Drop_Item_From_ContentBrowser" 1.0 1.0 0.0 0 0))

(event Custom|SetCameraRef
  (params (head :type Static%20Mesh%20Component%20Object%20Reference))
  ;[0.5477 0.8434 1] Set Refrences
  (Variables|Default|Sethead head))

(event Custom|SetControllerRef
  (params (Controller :type C%20Boxer%20Object%20Reference))
  ;[0.5477 0.8434 1] Set Refrences
  (Variables|refrences|SetControllerRef Controller))

(event EventTick
  (params (DeltaSeconds :type Float%20%28single-precision%29))
  (bind _controllerref (Variables|refrences|GetControllerRef))
  ;[1 0.4448 0.4448] PunchState
  (if (Utilities|Enum|Equal(Enum) (Variables|attackValues|Getstate) "NewEnumerator4")
    (CallFunction|SetPunch DeltaSeconds)
    (bind _isready (CallFunction|IsPunchSet))
    (if _isready
      (Variables|attackValues|Setstate "NewEnumerator0"))
    (elif (Utilities|Enum|Equal(Enum) (Variables|attackValues|Getstate) "NewEnumerator0")
      (CallFunction|Punch DeltaSeconds)
      (bind _isfinished (CallFunction|IsPunchFinished))
      (if _isfinished
        (Variables|attackValues|Setstate "NewEnumerator1"))
      (elif (Utilities|Enum|Equal(Enum) (Variables|attackValues|Getstate) "NewEnumerator1")
        (Utilities|FlowControl|Delay (Variables|attackValues|GettimeBetweenRetraction))
        (Variables|attackValues|Setstate "NewEnumerator2")
        (elif (Utilities|Enum|Equal(Enum) (Variables|attackValues|Getstate) "NewEnumerator2")
          (CallFunction|Retract DeltaSeconds)
          (bind _isfullyretracted (CallFunction|IsPunchFullyRetracted))
          (if _isfullyretracted
            (Variables|attackValues|Setstate "NewEnumerator3")
            (CallFunction|ResetPosition)
            (if (Utilities|IsValid _controllerref)
              (Variables|/Game/C_Boxer.C_Boxer_C|SetisAttacking _controllerref false)))
          (elif (Utilities|Enum|Equal(Enum) (Variables|attackValues|Getstate) "NewEnumerator3")
            _))))))

(event EventBeginPlay
  ;[1 1 1] Set retractSpeed
  (Variables|retract|SetretractSpeed (* (Variables|attackValues|GetpunchSpeed) -0.65))
  (Variables|retract|SetcameraReturnSpeed (* (Variables|Set|GetcameraMoveSpeed) -0.65)))

(fn Punch
  (params (time :type Float%20%28double-precision%29))
  (bind _punchspeed (Variables|attackValues|GetpunchSpeed))
  (bind _returnvalue (* time _punchspeed))
  (Transformation|AddLocalOffset (Variables|Default|Getfist) (Math|Vector|MakeVector 0.0 _returnvalue 0.0) true false)
  (Variables|positions|SettotalOffsetPunch (Math|Vector|MakeVector (.x (Variables|positions|GettotalOffsetPunch)) (+ _returnvalue (.y (Variables|positions|GettotalOffsetPunch))) (.z (Variables|positions|GettotalOffsetPunch)))))

(fn Retract
  (params (deltaTime :type Float%20%28double-precision%29))
  (bind _retractspeed (Variables|retract|GetretractSpeed))
  (bind _camerareturnspeed (Variables|retract|GetcameraReturnSpeed))
  (bind _returnvalue (* deltaTime _camerareturnspeed))
  (bind _returnvalue_2 (* deltaTime _retractspeed))
  (Transformation|AddLocalOffset (Variables|Default|Gethead) (Math|Vector|MakeVector 0.0 _returnvalue 0.0) true false)
  (Variables|positions|SetcameraOffset (Math|Vector|MakeVector (.x (Variables|positions|GetcameraOffset)) (+ _returnvalue (.y (Variables|positions|GetcameraOffset))) (.z (Variables|positions|GetcameraOffset))))
  (Transformation|AddLocalOffset (Variables|Default|Getfist) (Math|Vector|MakeVector 0.0 _returnvalue_2 0.0) true false)
  (Variables|positions|SettotalOffsetPunch (Math|Vector|MakeVector (.x (Variables|positions|GettotalOffsetPunch)) (+ _returnvalue_2 (.y (Variables|positions|GettotalOffsetPunch))) (.z (Variables|positions|GettotalOffsetPunch)))))

(fn IsPunchFinished
  (return (>= (.y (Variables|positions|GettotalOffsetPunch)) (Variables|attackValues|GetpunchDistance))))

(fn IsPunchFullyRetracted
  (return (<= (.y (Variables|positions|GettotalOffsetPunch)) 0.0)))

(fn ResetPosition
  (Transformation|AddLocalOffset (Variables|Default|Getfist) (Math|Vector|NegateVector (Variables|positions|GettotalOffsetPunch)) false true)
  (Variables|positions|SettotalOffsetPunch "0, 0, 0")
  (Transformation|AddLocalOffset (Variables|Default|Gethead) (Math|Vector|NegateVector (Variables|positions|GetcameraOffset)) false true)
  (Variables|positions|SetcameraOffset "0, 0, 0"))

(fn SetPunch
  (params (time :type Float%20%28double-precision%29))
  (bind _setspeed (Variables|Set|GetsetSpeed))
  (bind _cameramovespeed (Variables|Set|GetcameraMoveSpeed))
  (bind _returnvalue (* time _setspeed))
  (bind _returnvalue_2 (* time _cameramovespeed))
  ;[1 1 1] set camera offset
  (Transformation|AddLocalOffset (Variables|Default|Gethead) (Math|Vector|MakeVector 0.0 _returnvalue_2 0.0) true false)
  (Variables|positions|SetcameraOffset (Math|Vector|MakeVector (.x (Variables|positions|GetcameraOffset)) (+ _returnvalue_2 (.y (Variables|positions|GetcameraOffset))) (.z (Variables|positions|GetcameraOffset))))
  ;[1 1 1] set fist offset
  (Transformation|AddLocalOffset (Variables|Default|Getfist) (Math|Vector|MakeVector 0.0 _returnvalue 0.0) true false)
  (Variables|positions|SettotalOffsetPunch (Math|Vector|MakeVector (.x (Variables|positions|GettotalOffsetPunch)) (+ _returnvalue (.y (Variables|positions|GettotalOffsetPunch))) (.z (Variables|positions|GettotalOffsetPunch)))))

(fn IsPunchSet
  (return (<= (.y (Variables|positions|GettotalOffsetPunch)) (Variables|Set|GetsetDistance))))