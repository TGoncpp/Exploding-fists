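; Stamina component that holds a stamina pool, spends it on moves and loads player and opponent stamina bar widgets.
; GotEnoughStamina both checks and deducts a move's cost, or plays an invalid-action sound when stamina is short.
; Callers pass time into Regenerate, which can overshoot the maximum as it never clamps, and OffCenterPosition, which drains stamina down to zero.
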(event Custom|SetStamina
  (params (costOfMove :type Float%20%28double-precision%29))
  (Variables|Default|Setstamina (- (Variables|Default|Getstamina) costOfMove)))

(event Custom|LoadHud
  (bind _returnvalue (UserInterface|CreateWidget "/Game/HUD/HUD_PlayerStaminaBar.HUD_PlayerStaminaBar_C"))
  (UserInterface|Viewport|AddtoViewport _returnvalue 0)
  (bind _returnvalue_2 (UserInterface|CreateWidget "/Game/HUD/HUD_OppStaminaBar.HUD_OppStaminaBar_C"))
  (UserInterface|Viewport|AddtoViewport _returnvalue_2 0))

(fn GetStamina
  (return (Variables|Default|Getstamina)))

(fn GotEnoughStamina
  (params (cost :type Float%20%28double-precision%29))
  (if (>= (- (Variables|Default|Getstamina) cost) 0.0)
    (CallFunction|SetStamina cost)
    (return true)
    (else
      (Audio|PlaySound2D "/Engine/VREditor/Sounds/UI/Invalid_Action.Invalid_Action" 1.0 1.0 0.0 0 0)
      (return false))))

(fn Regenerate
  (params (time :type Float%20%28double-precision%29))
  (if (<= (Variables|Default|Getstamina) (Variables|Default|GetmaxStamina))
    (Variables|Default|Setstamina (+ (* (Variables|Default|GetregenerationRate) time) (Variables|Default|Getstamina)))))

(fn OffCenterPosition
  (params (time :type Float%20%28double-precision%29))
  (bind _output_get (Variables|Default|Setstamina (- (Variables|Default|Getstamina) (* time (Variables|Default|GetdegenerationRate)))))
  (if (< _output_get 0.0)
    (Variables|Default|Setstamina 0.0)))