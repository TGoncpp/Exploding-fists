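; Component that performs a straight punch by moving a fist and the head camera along local Y.
; Straight() starts a Tick-driven state machine: set the fist and camera, punch out to max distance, delay, then retract at speeds derived from the punch and camera speeds.
; Accumulated offsets decide phase changes and let ResetPosition teleport both back exactly, after which the controller's IsAttacking flag is cleared.
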(event Custom|Straight
  ;[1 0.3198 0.3198] Start attack
  (Variables|Default|Setstate "NewEnumerator4"))

(event Custom|SetHeadRef
  (params (cameraRef :type Static%20Mesh%20Component%20Object%20Reference))
  ;[0.5847 0.885 1] Set camera refrence
  (Variables|Default|Sethead cameraRef))

(event Custom|SetControllerRef
  (params (controllerRef :type C%20Boxer%20Object%20Reference))
  ;[0.5477 0.8434 1] Set Refrences
  (Variables|refrences|SetCOntrollerRef controllerRef))

(event Custom|InitStraight
  ;[1 1 1] Set retractSpeed
  (Variables|rettract|SetretractSpeed (* (Variables|attackValues|GetpunchSpeed) -0.65))
  (Variables|rettract|SetcameraReturnSpeed (* (Variables|set|GetcameraMoveSpeed) -0.65)))

(event EventTick
  (params (DeltaSeconds :type Float%20%28single-precision%29))
  (bind _controllerref (Variables|refrences|GetCOntrollerRef))
  ;[1 0.4448 0.4448] PunchState
  (if (Utilities|Enum|Equal(Enum) (Variables|Default|Getstate) "NewEnumerator4")
    (CallFunction|SetPunch DeltaSeconds)
    (bind _isset (CallFunction|IsPunchSet))
    (if _isset
      (Variables|Default|Setstate "NewEnumerator0"))
    (elif (Utilities|Enum|Equal(Enum) (Variables|Default|Getstate) "NewEnumerator0")
      (CallFunction|Punch DeltaSeconds)
      (bind _isfinished (CallFunction|IsPunchFinished))
      (if _isfinished
        (Variables|Default|Setstate "NewEnumerator1"))
      (elif (Utilities|Enum|Equal(Enum) (Variables|Default|Getstate) "NewEnumerator1")
        (Utilities|FlowControl|Delay (Variables|attackValues|GettimeBetweenRetraction))
        (Variables|Default|Setstate "NewEnumerator2")
        (elif (Utilities|Enum|Equal(Enum) (Variables|Default|Getstate) "NewEnumerator2")
          (CallFunction|Retract DeltaSeconds)
          (bind _isfullyretracted (CallFunction|IsPunchFullyRetracted))
          (if _isfullyretracted
            (Variables|Default|Setstate "NewEnumerator3")
            (CallFunction|ResetPosition)
            (if (Utilities|IsValid _controllerref)
              (Variables|/Game/C_Boxer.C_Boxer_C|SetisAttacking _controllerref false)))
          (elif (Utilities|Enum|Equal(Enum) (Variables|Default|Getstate) "NewEnumerator3")
            _))))))

(event EventBeginPlay
  ;[1 1 1] Set retractSpeed
  (Variables|rettract|SetretractSpeed (* (Variables|attackValues|GetpunchSpeed) -0.65))
  (Variables|rettract|SetcameraReturnSpeed (* (Variables|set|GetcameraMoveSpeed) -0.65)))

(fn Retract
  (params (deltaTime :type Float%20%28double-precision%29))
  (bind _camerareturnspeed (Variables|rettract|GetcameraReturnSpeed))
  (bind _retractspeed (Variables|rettract|GetretractSpeed))
  (bind _returnvalue (* deltaTime _camerareturnspeed))
  (bind _returnvalue_2 (* deltaTime _retractspeed))
  ;[1 1 1] Camera offset
  (Transformation|AddLocalOffset (Variables|Default|Gethead) (Math|Vector|MakeVector 0.0 _returnvalue 0.0) false false)
  (Variables|positions|SetcameraOffset (Math|Vector|MakeVector (.x (Variables|positions|GetcameraOffset)) (+ _returnvalue (.y (Variables|positions|GetcameraOffset))) (.z (Variables|positions|GetcameraOffset))))
  ;[1 1 1] fist offset
  (Transformation|AddLocalOffset (Variables|Default|Getfist) (Math|Vector|MakeVector 0.0 _returnvalue_2 0.0) true false)
  (Variables|positions|SettotalOffset (Math|Vector|MakeVector (.x (Variables|positions|GettotalOffset)) (+ _returnvalue_2 (.y (Variables|positions|GettotalOffset))) (.z (Variables|positions|GettotalOffset)))))

(fn IsPunchFullyRetracted
  (return (<= (.y (Variables|positions|GettotalOffset)) 0.0)))

(fn Punch
  (params (A :type Float%20%28double-precision%29))
  (bind _punchspeed (Variables|attackValues|GetpunchSpeed))
  (bind _returnvalue (* A _punchspeed))
  (Transformation|AddLocalOffset (Variables|Default|Getfist) (Math|Vector|MakeVector 0.0 _returnvalue 0.0) true false)
  (Variables|positions|SettotalOffset (Math|Vector|MakeVector (.x (Variables|positions|GettotalOffset)) (+ _returnvalue (.y (Variables|positions|GettotalOffset))) (.z (Variables|positions|GettotalOffset)))))

(fn IsPunchFinished
  (return (>= (.y (Variables|positions|GettotalOffset)) (Variables|attackValues|GetmaxPunchDistance))))

(fn ResetPosition
  (Transformation|AddLocalOffset (Variables|Default|Getfist) (Math|Vector|NegateVector (Variables|positions|GettotalOffset)) false true)
  (Variables|positions|SettotalOffset "0, 0, 0")
  (Transformation|AddLocalOffset (Variables|Default|Gethead) (Math|Vector|NegateVector (Variables|positions|GetcameraOffset)) false true)
  (Variables|positions|SetcameraOffset "0, 0, 0"))

(fn SetPunch
  (params (time :type Float%20%28double-precision%29))
  (bind _setspeed (Variables|set|GetsetSpeed))
  (bind _cameramovespeed (Variables|set|GetcameraMoveSpeed))
  (bind _returnvalue (* time _setspeed))
  (bind _returnvalue_2 (* time _cameramovespeed))
  (Transformation|AddLocalOffset (Variables|Default|Gethead) (Math|Vector|MakeVector 0.0 _returnvalue_2 0.0) true false)
  (Variables|positions|SetcameraOffset (Math|Vector|MakeVector (.x (Variables|positions|GetcameraOffset)) (+ _returnvalue_2 (.y (Variables|positions|GetcameraOffset))) (.z (Variables|positions|GetcameraOffset))))
  (Transformation|AddLocalOffset (Variables|Default|Getfist) (Math|Vector|MakeVector 0.0 _returnvalue 0.0) true false)
  (Variables|positions|SettotalOffset (Math|Vector|MakeVector (.x (Variables|positions|GettotalOffset)) (+ _returnvalue (.y (Variables|positions|GettotalOffset))) (.z (Variables|positions|GettotalOffset)))))

(fn IsPunchSet
  (return (<= (.y (Variables|positions|GettotalOffset)) (Variables|set|GetsetDistance))))